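; Level 2 anomaly actor that can be hidden or shown and keeps a scene component turned toward the player.
; Hide and Show events toggle the actor's hidden-in-game state.
; Each Tick it casts the player pawn to BP_FirstPersonCharacter, caches it, and uses FindLookAtRotation to rotate its Scene component to face that character's location.
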(event `Hide`
  (`self.SetActorHiddenInGame` true))

(event `Show`
  (`self.SetActorHiddenInGame` false))

(event `self.ReceiveTick`
  (params (DeltaSeconds :type "Float (single-precision)"))
  (bind _asbp_first_person_character (cast `/Game/FirstPerson/Blueprints/BP_FirstPersonCharacter` (`GameplayStatics.GetPlayerCharacter` 0)))
  (set `self.As BP First Person Character` _asbp_first_person_character)
  (`SceneComponent.K2_SetWorldRotation` (`self.Scene`) (`KismetMathLibrary.FindLookAtRotation` (`SceneComponent.K2_GetComponentLocation` (`self.Scene`)) (`self.K2_GetActorLocation` _asbp_first_person_character)) false false))

(fn `UserConstructionScript`)