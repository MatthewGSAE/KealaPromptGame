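; Post-processing controller that plays a world-healing screen fade, then loads the Parents_Home level.
; On BeginPlay it caches the first PostProcessVolume found in the level.
; HealWorld plays a timeline that drives the volume's BlendWeight, and each update also calls Play on a fade-out timeline writing the same weight.
; When the fade-out finishes, a short delay precedes the level change.
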(event `self.ReceiveBeginPlay`
  (bind _outactors (`GameplayStatics.GetAllActorsOfClass` "/Script/Engine.PostProcessVolume"))
  (set `self.NewVar_0` (`|GetArrayItem` _outactors)))

(event `HealWorld`
  (set `self.Blend Radius` (`PostProcessVolume.BlendRadius` (`self.NewVar_0`)))
  (bind (_direction _intensity) (`Timeline|WorldFade_TL`)
    (:`Update`
      (set `PostProcessVolume.BlendWeight` _intensity (`self.NewVar_0`))
      (bind (_direction_2 _fadeout) (`Timeline|Fadeoutgreen`)
        (:`Update`
          (set `PostProcessVolume.BlendWeight` _fadeout (`self.NewVar_0`)))
        (:`Finished`
          (`KismetSystemLibrary.Delay` 1.0)
          (`GameplayStatics.OpenLevel` "Parents_Home"))))))

(fn `UserConstructionScript`)