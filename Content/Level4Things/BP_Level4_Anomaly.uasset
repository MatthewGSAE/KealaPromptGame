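; Level 4 anomaly actor that the first-person player can interact with once it has been photographed.
; Tick turns on CanBeInteractedWith when HasBeenPhotographed is true.
; Box overlap tracks InRange and, for an interactable anomaly, shows or hides the player's interact widget and sets or clears the player's CurrentAnomalyInRange reference.
; The prompt is evaluated only on overlap events, using a player reference cached at BeginPlay.
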(event `self.ReceiveBeginPlay`
  (bind _asbp_first_person_character (cast `/Game/FirstPerson/Blueprints/BP_FirstPersonCharacter` (`GameplayStatics.GetPlayerCharacter` 0)))
  (set `self.As BP First Person Character` _asbp_first_person_character))

(event `self.ReceiveTick`
  (params (DeltaSeconds :type "Float (single-precision)"))
  (if (`self.has been photographed`)
    (set `self.CanBeInteractedWith` true)))

(event `self.Box.OnComponentBeginOverlap`
  (params (OverlappedComponent :type "PrimitiveComponent Object Reference") (OtherActor :type "Actor Object Reference") (OtherComp :type "PrimitiveComponent Object Reference") (OtherBodyIndex :type Integer) (bFromSweep :type Boolean) (SweepResult :type "HitResult Structure (by ref)"))
  (bind _as_bp_first_person_character (`self.As BP First Person Character`))
  (set `self.InRange?` true)
  (if (`self.CanBeInteractedWith`)
    (if (== OtherActor _as_bp_first_person_character)
      (`Widget.SetVisibility` (`/Game/FirstPerson/Blueprints/BP_FirstPersonCharacter.InteractWidget` _as_bp_first_person_character) "Visible")
      (set `/Game/FirstPerson/Blueprints/BP_FirstPersonCharacter.CurrentAnomalyInRange` self (`self.As BP First Person Character`)))))

(event `self.Box.OnComponentEndOverlap`
  (params (OverlappedComponent :type "PrimitiveComponent Object Reference") (OtherActor :type "Actor Object Reference") (OtherComp :type "PrimitiveComponent Object Reference") (OtherBodyIndex :type Integer))
  (bind _as_bp_first_person_character (`self.As BP First Person Character`))
  (set `self.InRange?` false)
  (if (`self.CanBeInteractedWith`)
    (if (== OtherActor _as_bp_first_person_character)
      (`Widget.SetVisibility` (`/Game/FirstPerson/Blueprints/BP_FirstPersonCharacter.InteractWidget` _as_bp_first_person_character) "Hidden")
      (set `/Game/FirstPerson/Blueprints/BP_FirstPersonCharacter.CurrentAnomalyInRange` null (`self.As BP First Person Character`)))))

(fn `UserConstructionScript`)